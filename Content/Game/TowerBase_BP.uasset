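; Tower defense turret Blueprint that auto-attacks Monster_BP enemies and can be upgraded or sold through a click-opened Towermenu.
; A timer-driven sphere trace gathers nearby monsters and picks a random Target, with reselection restarted when that target dies.
; While Level is at least 1, Tick aims TowerBase at the target and spawns bullets through a Delay, otherwise restoring its initial rotation.
; Upgrading swaps the mesh by Level, while selling resets Level and hides it.
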(event `重新检测`
  ;[1 1 1] 选择敌人
  (`KismetSystemLibrary.K2_SetTimerDelegate` (delegate `检测周围有无敌人`) 0.5 true :!label _label))

(event `self.ReceiveBeginPlay`
  (set `self.初始位置` (`KismetMathLibrary.Conv_RotatorToVector` (`SceneComponent.K2_GetComponentRotation` (`self.TowerBase`))))
  (goto _label))

(event `检测周围有无敌人`
  (bind _returnvalue (`self.K2_GetActorLocation`))
  (bind _monster_bp (`self.Monster BP`))
  ;[1 1 1] 选择敌人
  (`KismetArrayLibrary.Array_Clear` (`self.Monster BP`))
  (bind _outhits (`KismetSystemLibrary.SphereTraceMultiForObjects` _returnvalue _returnvalue 1000.0 (`|MakeArray` "ObjectTypeQuery3" :!type "EObjectTypeQuery Enum")))
  (for _array_element _outhits
    (bind _asmonster_bp (cast `/Game/Game/Monster_BP` (`.HitActor` (`GameplayStatics.BreakHitResult` _array_element))))
    (`KismetArrayLibrary.Array_Add` (`self.Monster BP`) _asmonster_bp))
  (if (not (== (`KismetArrayLibrary.Array_Length` (`self.Monster BP`)) 0))
    (set `self.target` (`|GetArrayItem` _monster_bp (`KismetMathLibrary.RandomIntegerInRange` 0 (- (`KismetArrayLibrary.Array_Length` _monster_bp) 1))))
    (`KismetSystemLibrary.K2_ClearAndInvalidateTimerHandle` (`self.choice`))))

(event `self.ReceiveTick`
  (params (DeltaSeconds :type "Float (single-precision)"))
  (if (>= (`self.Level`) 1)
    (`self.target`
      (:`then`
        (if (>= (`KismetMathLibrary.VSize` (- (`SceneComponent.K2_GetComponentLocation` (`self.TowerBase`)) (`self.K2_GetActorLocation` (`self.target`)))) 1000.0)
          ;[1 1 1] 转回
          (if (`self.已经转向`)
            (`self.转回`))
          (else
            ;[1 1 1] 怪物死亡销毁
            (if (`/Game/Game/Monster_BP.death` (`self.target`))
              (set `self.target` null)
              (`self.重新检测`)
              (else
                (set `self.已经转向` true)
                ;[1 1 1] 转向敌人
                (`SceneComponent.K2_SetWorldRotation` (`self.TowerBase`) (`KismetMathLibrary.FindLookAtRotation` (`SceneComponent.K2_GetComponentLocation` (`self.TowerBase`)) (`self.K2_GetActorLocation` (`self.target`))) false false)
                ;[1 1 1] 发射子弹
                (`KismetSystemLibrary.Delay` 0.5)
                (`self.target`
                  (:`then`
                    (`|SpawnActorFromClass` "/Game/Game/Bullet_TowerBase_BP.Bullet_TowerBase_BP_C" (`KismetMathLibrary.Conv_VectorToTransform` (`SceneComponent.K2_GetComponentLocation` (`self.TowerBase`))) "Undefined" "OverrideRootScale" null (`self.target`) null))
                  (:`else`)))))))
      (:`else`
        ;[1 1 1] 转向回到初始化
        (if (`self.已经转向`)
          (set `self.已经转向` false :!label _label_2)
          (`SceneComponent.K2_SetWorldRotation` (`self.TowerBase`) (`KismetMathLibrary.Conv_VectorToRotator` (`self.初始位置`)) false false))))))

(event `转回`
  ;[1 1 1] 转向回到初始化
  (goto _label_2))

(event `self.ReceiveActorOnClicked`
  (params (ButtonPressed :type "Key Structure"))
  ;[1 1 1] 防御塔操作菜单
  (bind _foundwidgets (`WidgetBlueprintLibrary.GetAllWidgetsOfClass` "/Game/Game/UI/Towermenu.Towermenu_C"))
  (for _array_element _foundwidgets
    (`Widget.RemoveFromParent` _array_element))
  (set `self.菜单已经出现` true)
  (bind _returnvalue (`|CreateWidget` "/Game/Game/UI/Towermenu.Towermenu_C" null (`self.Level`) self))
  (`UserWidget.AddToViewport` _returnvalue 0)
  (bind _returnvalue_2 (`WidgetLayoutLibrary.GetMousePositionOnViewport`))
  (`UserWidget.SetPositionInViewport` _returnvalue _returnvalue_2 false))

(event `升级`
  ;[1 1 1] 防御塔升级
  (`/Engine/EditorBlueprintResources/StandardMacros.IncrementInt` (`self.Level`)
    (:`  `
      (`SceneComponent.SetVisibility` (`self.TowerBase`) true false)
      (`SkinnedMeshComponent.SetSkinnedAssetAndUpdate` (`self.TowerBase`) (select `int` (`self.Level`) :`0` null :`1` "/Game/CSC/Meshes/SK_RLV_Base1.SK_RLV_Base1" :`2` "/Game/CSC/Meshes/SK_TANK_Base1.SK_TANK_Base1" :`3` "/Game/CSC/Meshes/TowerBase1.TowerBase1" :`4` "/Game/CSC/Meshes/SK_CSC_Body1.SK_CSC_Body1" :`5` "/Game/CSC/Meshes/SK_CSC_Body1.SK_CSC_Body1" :!type "SkeletalMesh Object Reference") true))))

(event `售出`
  ;[1 1 1] 卖塔
  (set `self.Level` 0)
  (`SceneComponent.SetVisibility` (`self.TowerBase`) false false))

(fn `UserConstructionScript`)