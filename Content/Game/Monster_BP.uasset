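; Tower defense monster that walks a path from its birth point and costs the player health if it reaches the end.
; After a short start delay, it follows linked path points with AI MoveTo, each point supplying the next.
; When the chain ends, it subtracts Damage from GameBlood in GameMode_TD and destroys itself.
; Incoming damage lowers Blood; at zero it flags Death, simulates mesh physics and is destroyed after a delay.
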(event `self.ReceiveBeginPlay`
  (bind _asgame_mode_td (cast `/Game/Game/GameMode_TD` (`GameplayStatics.GetGameMode`) :!pure true))
  ;[1 1 1] 生成于出生点，消失于终点，自动行走路径, 扣除玩家血量
  (`KismetSystemLibrary.Delay` 0.2)
  (set `self.PathPointNext` (`/Game/Game/BirthPoint_BP.PathPointFir` (`self.BirthPoint`)))
  (`|AIMoveTo` self (0.0 0.0 0.0) (`self.PathPointNext`) :!label _label
    (:`OnSuccess`
      (set `self.PathPointNext` (`/Game/Game/PathPoint_BP.PathPoint` (`self.PathPointNext`)))
      (`self.PathPointNext`
        (:`then`
          (goto _label))
        (:`else`
          (set `/Game/Game/GameMode_TD.GameBlood` (- (`/Game/Game/GameMode_TD.GameBlood` _asgame_mode_td) (`self.damage`)) _asgame_mode_td)
          (`self.K2_DestroyActor` self))))))

(event `self.ReceiveAnyDamage`
  (params (Damage :type "Float (single-precision)") (DamageType :type "DamageType Object Reference") (InstigatedBy :type "Controller Object Reference") (DamageCauser :type "Actor Object Reference"))
  (bind _output_get (set `self.Blood` (- (`self.Blood`) Damage)))
  (if (<= _output_get 0.0)
    (set `self.death` true)
    (`PrimitiveComponent.SetSimulatePhysics` (`self.Mesh`) true)
    (`KismetSystemLibrary.Delay` 2.0)
    (`self.K2_DestroyActor`)))

(fn `UserConstructionScript`)