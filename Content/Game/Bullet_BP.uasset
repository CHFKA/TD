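; Bullet_BP is a homing projectile that chases its Bullettarget actor and damages monsters on contact.
; Each tick it sets the ProjectileMovement velocity at a fixed speed from the look-at direction toward the target, passed as a local-space velocity.
; When its Box overlaps a Monster_BP, it applies a fixed amount of damage and destroys itself.
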(event `self.ReceiveTick`
  (params (DeltaSeconds :type "Float (single-precision)"))
  (`ProjectileMovementComponent.SetVelocityInLocalSpace` (`self.ProjectileMovement`) (* (`KismetMathLibrary.Conv_RotatorToVector` (`KismetMathLibrary.FindLookAtRotation` (`self.K2_GetActorLocation`) (`self.K2_GetActorLocation` (`self.bullettarget`)))) 2500.0)))

(event `self.Box.OnComponentBeginOverlap`
  (params (OverlappedComponent :type "PrimitiveComponent Object Reference") (OtherActor :type "Actor Object Reference") (OtherComp :type "PrimitiveComponent Object Reference") (OtherBodyIndex :type Integer) (bFromSweep :type Boolean) (SweepResult :type "HitResult Structure (by ref)"))
  (bind _asmonster_bp (cast `/Game/Game/Monster_BP` OtherActor))
  (`GameplayStatics.ApplyDamage` _asmonster_bp 10.0)
  (`self.K2_DestroyActor`))

(fn `UserConstructionScript`)